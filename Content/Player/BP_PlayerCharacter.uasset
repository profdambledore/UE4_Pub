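; BP_PlayerCharacter is the player character Blueprint, and its logic here sets up and controls the player's on-screen UI.
; On BeginPlay it creates the player HUD and money text widgets, adds both to the viewport and passes itself to the HUD as the player reference.
; A SwapUIIndex event changes the visible HUD page by setting the active index of the HUD's widget switcher.
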(event EventBeginPlay
  (bind _self self)
  (bind _returnvalue (Game|ConstructObjectfromClass "/Game/Player/UI/WBP_PlayerHUD.WBP_PlayerHUD_C" self))
  (bind _output_get (Variables|Default|SetHUD _returnvalue))
  (UserInterface|Viewport|AddtoViewport _output_get 0)
  (Default|GetPlayerRef _output_get _self)
  (bind _returnvalue_2 (Game|ConstructObjectfromClass "/Game/Player/UI/WBP_MoneyText.WBP_MoneyText_C" _self))
  (bind _output_get_2 (Variables|Default|SetMoneeHud _returnvalue_2))
  (UserInterface|Viewport|AddtoViewport _output_get_2 0))

(event EventSwapUIIndex
  (params (NewIndex :type Integer))
  (Class|WidgetSwitcher|SetActiveWidgetIndex (Variables|/Game/Player/UI/WBP_PlayerHUD.WBP_PlayerHUD_C|GetSwitcher (Variables|Default|GetHUD)) NewIndex))

(fn ConstructionScript)